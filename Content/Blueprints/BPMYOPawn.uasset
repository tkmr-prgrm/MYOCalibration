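; Pawn that connects a Myo armband and sets up EMG-based calibration for fist and finger-spread gestures.
; BeginPlay adds the Myo component, the first pose event enables EMG streaming with a vibration, and EMG events store raw data.
; Input actions flag calibration start, while custom events sum absolute per-channel samples for later averaging.
; Nothing here calls those events, and the pose checks and data clearing are stubs.
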(event Custom|SpreadCalibrate
  ;[1 1 1] カスタムイベント
  ;;[1 1 1] SpreadCalibrate Spreadしている時のEMGDataの平均をとる
  (Math|Integer|IncrementInt (Variables|Default|GetaddCount)
    (:%20%20
      (for (_array_element _array_index) (Utilities|Struct|BreakMyoEmgData (Variables|Default|GetrawEMGData))
        (Utilities|Array|SetArrayElem (Variables|Default|GetspreadCalibrateData) _array_index (+ (Math|Integer|Absolute(Integer) _array_element) (Utilities|Array|Get(acopy) (Variables|Default|GetspreadCalibrateData) _array_index)))))))

(event Custom|FistCalibrate
  ;[1 1 1] カスタムイベント
  ;;[1 1 1] FistCalibrate Fistしている時のEMGDataの平均をとる
  (Math|Integer|IncrementInt (Variables|Default|GetaddCount)
    (:%20%20
      (for (_array_element _array_index) (Utilities|Struct|BreakMyoEmgData (Variables|Default|GetrawEMGData))
        (Utilities|Array|SetArrayElem (Variables|Default|GetfistCalibrateData) _array_index (+ (Math|Integer|Absolute(Integer) _array_element) (Utilities|Array|Get(acopy) (Variables|Default|GetfistCalibrateData) _array_index)))))))

(event EventBeginPlay
  ;[0 0.1254 1] BeginPlay
  ;;[1 1 1] MyoComponent追加変数作成
  (bind _returnvalue (AddComponent|AddMyoComponent))
  (Variables|Default|SetMyo _returnvalue))

(event EventTick
  (params (DeltaSeconds :type Float%20%28single-precision%29)))

(event EventOnEmgData
  (params (myo :type Myo%20Controller%20Object%20Reference) (data :type Myo%20Emg%20Data%20Structure))
  (Variables|Default|SetrawEMGData data))

(event EventOnPose
  (params (myo :type Myo%20Controller%20Object%20Reference) (pose :type MyoPose%20Enum))
  ;[0 0.7959 1] MyoOnPose
  (if (not (Variables|Default|GetbSetEMG))
    (Variables|Default|SetMyoController myo)
    ;;[1 1 1] EMGDataを取得
    (switch Utilities|FlowControl|Switch|SwitchonMyoPose pose
      (:MYO_POSE_REST
        _)
      (:MYO_POSE_FIST
        _)
      (:MYO_POSE_WAVEIN
        _)
      (:MYO_POSE_WAVEOUT
        _)
      (:MYO_POSE_FINGERSPREAD
        _)
      (:MYO_POSE_DOUBLETAP
        _)
      (:MYO_POSE_UNKNOWN
        _))
    (Class|MyoController|SetStreamEmg (Variables|Default|GetMyoController) "MYO_STREAM_EMG_ENABLED")
    (Class|MyoController|VibrateDevice (Variables|Default|GetMyoController) "MYO_VIBRATION_SHORT")
    (Variables|Default|SetbSetEMG true)))

(event Input|ActionEvents|InputActionFistCalibrate
  ;[1 1 1] Input
  ;;[0 1 0.391] FistCalibrate
  (:Pressed
    (if (not (Variables|Default|GetbCalibrateNow))
      (Variables|Default|SetbCalibrateNow true)
      (if (not (Variables|Default|GetbDoneFistCalibrate))
        (Variables|Default|SetbFistCalibrateNow true)
        (Variables|Default|SetcalibrateStartTime (Utilities|Time|GetRealTimeSeconds))))))

(event Input|ActionEvents|InputActionSpreadCalibrate
  ;[1 1 1] Input
  ;;[0 1 0.1407] SpreadCalibrate
  (:Pressed
    (if (not (Variables|Default|GetbCalibrateNow))
      (Variables|Default|SetbCalibrateNow true)
      (if (not (Variables|Default|GetbDoneSpreadCalibrate))
        (Variables|Default|SetbSpreadCalibrateNow true)
        (Variables|Default|SetcalibrateStartTime (Utilities|Time|GetRealTimeSeconds))))))

(event Input|ActionEvents|InputActionClearCalibrateData
  ;[1 1 1] Input
  ;;[0 1 0.9016] ClearCalibrationData
  (:Pressed
    (CallFunction|ClearCalibrateData)
    (Development|PrintString "ClearCalibrationData")))

(fn ConstructionScript)

(fn FistCheck
  (params (EMGData :type Array%20of%20Integers))
  (return false))

(fn SpreadCheck
  (params (EMGData :type Array%20of%20Integers))
  (return false))

(fn RestCheck
  (params (EMGData :type Array%20of%20Integers))
  (return false))

(fn ClearCalibrateData)